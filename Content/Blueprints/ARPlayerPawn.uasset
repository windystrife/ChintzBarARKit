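; AR player pawn that places one fishing scene, goldfish or portal on a detected surface by touch, on non-Android platforms only.
; Tick drives main-widget prompts from tracking quality, assuming a plane exists off Android, and prints debug info.
; Touch runs an ARKit hit test, then spawns per widget selection or moves existing portals, yawed from the view direction.
; FishGoldSpawn checks weekend-afternoon and GPS bounds but is uncalled here; location setup is unwired.
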(fn ConstructionScript)

(fn DetermineTrackingQuality
  ;[1 1 1] If we haven't found any planes yet, downgrade the tracking quality by 1 notch.
  (bind _returnvalue (Class|ARBlueprintFunctionLibrary|GetTrackingQuality))
  (bind _output_get (LocalVariables|SetTrackingQuality _returnvalue))
  (Variables|Default|Settrackquality_public (select (>= (Variables|Default|GetnumPlanesDetected) 1) _output_get (Utilities|Select :Index _output_get :NotAvailable "NotAvailable" :Limited "Limited" :Normal "Limited")))
  (return (select (>= (Variables|Default|GetnumPlanesDetected) 1) _output_get (Utilities|Select :Index _output_get :NotAvailable "NotAvailable" :Limited "Limited" :Normal "Limited"))))

(fn DoHitTestforARKIT
  (params (InputPin :type Vector%202D%20Structure) (Player :type Player%20Controller%20Object%20Reference))
  (bind (_outresults _returnvalue) (Class|AppleARKitBlueprintLibrary|HitTestatScreenPositionTrackingSpace InputPin "ExistingPlane"))
  (if _returnvalue
    (Development|PrintString (Utilities|String|Append "HIT from :  " (Utilities|String|ToString(Vector2d) InputPin) " Distance : " (Utilities|String|ToString(Float) (.Distance (Utilities|Struct|BreakAppleARKitHitTestResult (Utilities|Array|Get(acopy) _outresults))))) true true "(R=0.707400,G=1.000000,B=0.000000,A=1.000000)")
    (Development|PrintString (Utilities|String|ToString(Transform) (.Transform (Utilities|Struct|BreakAppleARKitHitTestResult (Utilities|Array|Get(acopy) _outresults)))) true true "(R=1.000000,G=0.965410,B=0.000000,A=1.000000)")
    (return true (Math|Transform|MakeTransform (.Location (Math|Transform|BreakTransform (.Transform (Utilities|Struct|BreakAppleARKitHitTestResult (Utilities|Array|Get(acopy) _outresults))))) (Math|Rotator|MakeRotator (.Roll (Math|Rotator|BreakRotator (Math|Rotator|FindLookatRotation (.Location (Math|Transform|BreakTransform (.Transform (Utilities|Struct|BreakAppleARKitHitTestResult (Utilities|Array|Get(acopy) _outresults))))) (+ (.Location (Math|Transform|BreakTransform (.Transform (Utilities|Struct|BreakAppleARKitHitTestResult (Utilities|Array|Get(acopy) _outresults))))) (Math|Vector|Normalize (* (.WorldDirection (Class|GameplayStatics|DeprojectScreentoWorld Player InputPin)) "1.000000,1.000000, 0")))))) (.Pitch (Math|Rotator|BreakRotator (Math|Rotator|FindLookatRotation (.Location (Math|Transform|BreakTransform (.Transform (Utilities|Struct|BreakAppleARKitHitTestResult (Utilities|Array|Get(acopy) _outresults))))) (+ (.Location (Math|Transform|BreakTransform (.Transform (Utilities|Struct|BreakAppleARKitHitTestResult (Utilities|Array|Get(acopy) _outresults))))) (Math|Vector|Normalize (* (.WorldDirection (Class|GameplayStatics|DeprojectScreentoWorld Player InputPin)) "1.000000,1.000000, 0")))))) (- (.Yaw (Math|Rotator|BreakRotator (Math|Rotator|FindLookatRotation (.Location (Math|Transform|BreakTransform (.Transform (Utilities|Struct|BreakAppleARKitHitTestResult (Utilities|Array|Get(acopy) _outresults))))) (+ (.Location (Math|Transform|BreakTransform (.Transform (Utilities|Struct|BreakAppleARKitHitTestResult (Utilities|Array|Get(acopy) _outresults))))) (Math|Vector|Normalize (* (.WorldDirection (Class|GameplayStatics|DeprojectScreentoWorld Player InputPin)) "1.000000,1.000000, 0")))))) -9e+01)) (.Scale (Math|Transform|BreakTransform (.Transform (Utilities|Struct|BreakAppleARKitHitTestResult (Utilities|Array|Get(acopy) _outresults)))))) (Math|Transform|MakeTransform (.Location (Math|Transform|BreakTransform (.Transform (Utilities|Struct|BreakAppleARKitHitTestResult (Utilities|Array|Get(acopy) _outresults))))) (Math|Rotator|MakeRotator (.Roll (Math|Rotator|BreakRotator (Math|Rotator|FindLookatRotation (.Location (Math|Transform|BreakTransform (.Transform (Utilities|Struct|BreakAppleARKitHitTestResult (Utilities|Array|Get(acopy) _outresults))))) (+ (.Location (Math|Transform|BreakTransform (.Transform (Utilities|Struct|BreakAppleARKitHitTestResult (Utilities|Array|Get(acopy) _outresults))))) (Math|Vector|Normalize (* (.WorldDirection (Class|GameplayStatics|DeprojectScreentoWorld Player InputPin)) "1.000000,1.000000, 0")))))) (.Pitch (Math|Rotator|BreakRotator (Math|Rotator|FindLookatRotation (.Location (Math|Transform|BreakTransform (.Transform (Utilities|Struct|BreakAppleARKitHitTestResult (Utilities|Array|Get(acopy) _outresults))))) (+ (.Location (Math|Transform|BreakTransform (.Transform (Utilities|Struct|BreakAppleARKitHitTestResult (Utilities|Array|Get(acopy) _outresults))))) (Math|Vector|Normalize (* (.WorldDirection (Class|GameplayStatics|DeprojectScreentoWorld Player InputPin)) "1.000000,1.000000, 0")))))) (+ (.Yaw (Math|Rotator|BreakRotator (Math|Rotator|FindLookatRotation (.Location (Math|Transform|BreakTransform (.Transform (Utilities|Struct|BreakAppleARKitHitTestResult (Utilities|Array|Get(acopy) _outresults))))) (+ (.Location (Math|Transform|BreakTransform (.Transform (Utilities|Struct|BreakAppleARKitHitTestResult (Utilities|Array|Get(acopy) _outresults))))) (Math|Vector|Normalize (* (.WorldDirection (Class|GameplayStatics|DeprojectScreentoWorld Player InputPin)) "1.000000,1.000000, 0")))))) 1.8e+02)) (.Scale (Math|Transform|BreakTransform (.Transform (Utilities|Struct|BreakAppleARKitHitTestResult (Utilities|Array|Get(acopy) _outresults)))))))
    (else
      (return false "" ""))))

(fn CachePlatform
  ;[1 1 1] Cache platform that we're running on for switching on platform-specific functionality
  (bind _returnvalue (Game|GetPlatformName))
  (bind _output_get (Variables|Default|SetbIsAndroid (Utilities|Enum|Equal(Enum) _returnvalue "Android")))
  (Development|PrintString _returnvalue)
  (Development|PrintString (Utilities|String|ToString(Boolean) _output_get)))

(fn DisplayDebugTrackingInfo
  ;[1 1 1] Display Debug Tracking Info
  (Development|PrintString (Utilities|String|ToString(Transform) (Transformation|GetWorldTransform (Variables|/Script/Engine.PlayerCameraManager|GetTransformComponent (Game|GetPlayerCameraManager 0)))) true false "(R=0.081168,G=1.000000,B=0.218801,A=1.000000)" 0.0)
  (bind _tracking (CallFunction|DetermineTrackingQuality))
  (Development|PrintString (Utilities|String|Append "[ " (Utilities|String|EnumtoString _tracking) " ]") true false (Utilities|Select :Index _tracking :NotAvailable "(R=1.000000,G=0.000000,B=0.158961,A=1.000000)" :Limited "(R=1.000000,G=0.226966,B=0.000000,A=1.000000)" :Normal "(R=0.283149,G=1.000000,B=0.000000,A=1.000000)") 0.0))

(fn FishGoldSpawn?
  (bind _latitude (Variables|Default|GetLatitude))
  (bind _longitude (Variables|Default|GetLongitude))
  (bind _returnvalue (<= _longitude -4.377846))
  (bind _returnvalue_2 (<= _latitude 50.459433))
  (bind _returnvalue_3 (>= _latitude 50.45885))
  (bind _returnvalue_4 (>= _longitude -4.377999))
  (bind _returnvalue_5 (and _returnvalue_2 _returnvalue_3))
  (bind _returnvalue_6 (and _returnvalue _returnvalue_4))
  (bind _returnvalue_7 (and _returnvalue_5 _returnvalue_6))
  (LocalVariables|SetDateTime (Math|DateTime|Now))
  (bind _returnvalue_8 (Class|WeekDay|WeekDay (.Year (Math|DateTime|BreakDateTime (LocalVariables|GetDateTime))) (.Month (Math|DateTime|BreakDateTime (LocalVariables|GetDateTime))) (.Day (Math|DateTime|BreakDateTime (LocalVariables|GetDateTime)))))
  (if (and (or (== _returnvalue_8 7) (== _returnvalue_8 1)) (and (<= (.Hour (Math|DateTime|BreakDateTime (LocalVariables|GetDateTime))) 24) (> (.Hour (Math|DateTime|BreakDateTime (LocalVariables|GetDateTime))) 12)))
    (if _returnvalue_7
      (return true true true)
      (else
        (return false true false)))
    (elif _returnvalue_7
      (return true false false)
      (else
        (return false false false)))))

(fn Portal1Teleport)

(event EventBeginPlay
  (Utilities|FlowControl|Sequence
    (:then_0
      (CallFunction|CachePlatform)
      (bind _returnvalue (UserInterface|CreateWidget "/Game/Blueprints/Widget/MainWidget.MainWidget_C"))
      (UserInterface|Viewport|AddtoViewport _returnvalue 0)
      (Variables|Default|SetMaiNWidget _returnvalue))
    (:then_1
      (Actor|GetAllActorsOfClass 0))))

(event EventTick
  (params (DeltaSeconds :type Float%20%28single-precision%29))
  (bind _mainwidget (Variables|Default|GetMaiNWidget))
  (Utilities|FlowControl|Sequence
    (:then_0
      ;[0 0 0] Display Debug Information About Found Planes
      (if (not (Variables|Default|GetbIsAndroid))
        ;;[0.156 0.5013 1 0.3] ARKit : detects planes quickly enough to just assume it found one if the tracking is good
        (Variables|Default|SetnumPlanesDetected 1)))
    (:then_1
      (CallFunction|DisplayDebugTrackingInfo))
    (:then_2
      (if (Variables|Default|Getspawnactor)
        (Widget|SetVisibility (Variables|/Game/Blueprints/Widget/MainWidget.MainWidget_C|GetStatus_FloorDectect (Variables|Default|GetMaiNWidget)) "Collapsed")
        (|Show_UI_GoldFish)
        (if (Variables|/Game/Blueprints/Widget/MainWidget.MainWidget_C|GetHomeActive? (Variables|Default|GetMaiNWidget))
          (Variables|/Game/Blueprints/Widget/MainWidget.MainWidget_C|SetCameraActive? _mainwidget false)
          (else
            (Variables|/Game/Blueprints/Widget/MainWidget.MainWidget_C|SetCameraActive? _mainwidget true)))
        (else
          (bind _output_get (Variables|Default|Settext (Utilities|String|EnumtoString (Variables|Default|Gettrackquality_public))))
          (if (Utilities|Enum|Equal(Enum) _output_get "Normal")
            (Variables|Default|Setcanspawn?? true)
            (if (== (Variables|/Game/Blueprints/Widget/MainWidget.MainWidget_C|GetBackGround (Variables|Default|GetMaiNWidget)) 5)
              (Rendering|Components|TextRender|SetText (Variables|/Game/Blueprints/Widget/MainWidget.MainWidget_C|GetTextTest (Variables|Default|GetMaiNWidget)) "Plane Dectected Touch On The Screen To Place Portal")
              (else
                (Rendering|Components|TextRender|SetText (Variables|/Game/Blueprints/Widget/MainWidget.MainWidget_C|GetTextTest (Variables|Default|GetMaiNWidget)) "Plane Dectected Please Touch On The Screen For Fishing")))
            (else
              (Variables|Default|Setcanspawn?? false)
              (Rendering|Components|TextRender|SetText (Variables|/Game/Blueprints/Widget/MainWidget.MainWidget_C|GetTextTest (Variables|Default|GetMaiNWidget)) "Searching for surfaces..."))))))
    (:then_3
      (if (and (Variables|Default|Getspawnactor) (== (Variables|/Game/Blueprints/Widget/MainWidget.MainWidget_C|GetBackGround (Variables|Default|GetMaiNWidget)) 5))
        (Widget|SetVisibility (Variables|/Game/Blueprints/Widget/MainWidget.MainWidget_C|GetCameraUI_Selfie1 (Variables|Default|GetMaiNWidget)) "Visible")))))

(event Input|TouchEvents|InputTouch
  (params (Location :type Vector) (FingerIndex :type ETouchIndex%20Enum))
  (bind _returnvalue (Game|GetPlayerController 0))
  (bind _mainwidget (Variables|Default|GetMaiNWidget))
  (bind (_locationx _locationy) (Class|PlayerController|GetInputTouchState _returnvalue FingerIndex))
  (bind _returnvalue_2 (Math|Vector2D|MakeVector2D _locationx _locationy))
  (:Pressed
    ;[0 0 0] ARCore and ARKit currently have differences in plane detection as well as how they expect Actors to be placed in the world, so we account for that here. Expect updates that simplify this in future releases
    (if (not (Variables|Default|GetbIsAndroid))
      ;;[1 1 1] IOS
      (if (not (Variables|Default|Getspawnactor))
        (bind (_success _spawntransform _spawnportal) (CallFunction|DoHitTestforARKIT _returnvalue_2 _returnvalue))
        (if _success
          (if (Variables|/Game/Blueprints/Widget/MainWidget.MainWidget_C|GetSpawnGoldFish (Variables|Default|GetMaiNWidget))
            (Game|SpawnActorfromClass "/Game/Blueprints/BP_PlaceableGOldFish.BP_PlaceableGOldFish_C" _spawntransform "AlwaysSpawn" 0 0)
            (Variables|Default|Setspawnactor true)
            (else
              (switch int (Variables|/Game/Blueprints/Widget/MainWidget.MainWidget_C|GetBackGround (Variables|Default|GetMaiNWidget))
                (:1
                  (Game|SpawnActorfromClass "/Game/Blueprints/ARKIT/ChintzFishCurtain1.ChintzFishCurtain1_C" _spawntransform "AlwaysSpawn" 0 0)
                  (Variables|Default|Setspawnactor true))
                (:2
                  (Game|SpawnActorfromClass "/Game/Blueprints/ARKIT/ChintzFishCurtain2.ChintzFishCurtain2_C" _spawntransform "Undefined" 0 0)
                  (Variables|Default|Setspawnactor true))
                (:3
                  (Game|SpawnActorfromClass "/Game/Blueprints/ARKIT/ChintzFishCurtain3.ChintzFishCurtain3_C" _spawntransform "Undefined" 0 0)
                  (Variables|Default|Setspawnactor true))
                (:4
                  (Game|SpawnActorfromClass "/Game/Blueprints/ARKIT/ChintzFishNoCurtain.ChintzFishNoCurtain_C" _spawntransform "Undefined" 0 0)
                  (Variables|Default|Setspawnactor true)
                  (if (not (Variables|/Game/Blueprints/Widget/MainWidget.MainWidget_C|GetLogin?? _mainwidget))
                    (Widget|SetVisibility (Variables|/Game/Blueprints/Widget/MainWidget.MainWidget_C|GetNoLoginGoldFish_Message _mainwidget) "Visible")))
                (:5
                  (bind _outactors (Actor|GetAllActorsOfClass "/Game/Blueprints/Portal/Portal1_BP.Portal1_BP_C"))
                  (for _array_element _outactors
                    (Transformation|SetActorTransform _array_element _spawnportal)
                    (Transformation|SetActorTransform _array_element _spawnportal)
                    (Variables|Default|Setspawnactor true)
                    (Variables|Default|SetPortal1_SpawnTransform _spawnportal))
                  (bind _outactors_2 (Actor|GetAllActorsOfClass "/Game/Blueprints/Portal/Portal2_BP.Portal2_BP_C"))
                  (for _array_element_2 _outactors_2
                    (Transformation|SetActorRotation _array_element_2 (Math|Rotator|MakeRotator (.roll (Transformation|GetActorRotation _array_element_2)) (.pitch (Transformation|GetActorRotation _array_element_2)) (+ (.yaw (.Rotation (Math|Transform|BreakTransform (Variables|Default|GetPortal1_SpawnTransform)))) 1.8e+02))))))))
          (else
            ;[1 -0.7571 -1.971] No Hit Info Found
            (Development|PrintString (Utilities|String|Append "NO HIT" (Utilities|String|ToString(Vector2d) _returnvalue_2)) true true "(R=1.000000,G=0.000000,B=0.356152,A=1.000000)" 1.0)))))))