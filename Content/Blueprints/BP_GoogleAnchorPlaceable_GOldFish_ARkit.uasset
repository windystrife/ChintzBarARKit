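; An AR placeable actor, named as a goldfish, built around a Google ARCore anchor and an attached plane.
; HandleVisibility hides it when tracking stops, follows subsumed planes, and snaps its height to the plane.
; GetDayOfWeek computes a weekday from a date arithmetically.
; Event graph events are empty, nothing here calls HandleVisibility, and the anchor setup and location-services logic are disconnected, so never run.
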(event EventBeginPlay)

(event Collision|EventActorBeginOverlap
  (params (OtherActor :type Actor%20Object%20Reference)))

(event EventTick
  (params (DeltaSeconds :type Float%20%28single-precision%29)))

(fn ConstructionScript)

(fn HandleVisibility
  (params (Delta :type Float%20%28single-precision%29))
  (bind _returnvalue (Transformation|GetActorLocation))
  (bind (_x _y) (Math|Vector|BreakVector _returnvalue))
  (if (CallFunction|GetifStoppedTracking)
    (Rendering|SetActorHiddenInGame true)
    (else
      (|CallParentFunction Delta)
      (if (Utilities|IsValid (Variables|Default|GetAttachedPlane))
        (Utilities|FlowControl|Sequence
          (:then_0
            ;[1 1 1] Update attached plane if the plane is subsumed
            (if (Utilities|Enum|Equal(Enum) (Class|GoogleARCorePlane|GetTrackingState (Variables|Default|GetAttachedPlane)) "Subsumed")
              (Variables|Default|SetAttachedPlane (Class|GoogleARCorePlane|GetSubsumedby (Variables|Default|GetAttachedPlane)))))
          (:then_1
            ;[1 1 1] Toggle the Actor visibility based on the plane tracking status as well
            (if (Utilities|Enum|Equal(Enum) (Class|GoogleARCoreAnchorBase|GetTrackingState (Class|GoogleARCoreAnchorActor|GetARAnchor (Variables|Default|GetAnchorActor))) "Tracking")
              (Rendering|SetActorHiddenInGame (Utilities|Select :Index (Class|GoogleARCorePlane|GetTrackingState (Variables|Default|GetAttachedPlane)) :Tracking false :Subsumed true :NotCurrentlyTracking true :StoppedTracking true))))
          (:then_2
            ;[1 1 1] Adjust tne Anchor Actor Z position using the attached plane
            (Transformation|SetActorLocation (Math|Vector|MakeVector _x _y (.Z (Math|Vector|BreakVector (.location (Class|GoogleARCorePlane|GetBoundingBoxWorldTransform (Variables|Default|GetAttachedPlane)))))) false false)))))))

(fn GetifStoppedTracking
  (bind _attachedplane (Variables|Default|GetAttachedPlane))
  (return (or (Utilities|Enum|Equal(Enum) (Class|GoogleARCoreAnchorBase|GetTrackingState (Class|GoogleARCoreAnchorActor|GetARAnchor (Variables|Default|GetAnchorActor))) "StoppedTracking") (and (Utilities|IsValid _attachedplane) (Utilities|Enum|Equal(Enum) (Class|GoogleARCorePlane|GetTrackingState _attachedplane) "StoppedTracking")))))

(fn GetDayOfWeek
  (params (Day :type Integer) (Month :type Integer) (Year :type Integer))
  (LocalVariables|SetDayTemp Day)
  (LocalVariables|SetMonthTemp Month)
  (LocalVariables|SetYearTemp Year)
  (if (< Month 3)
    (LocalVariables|SetMonthTemp (+ (LocalVariables|GetMonthTemp) 12))
    (LocalVariables|SetYearTemp (- (LocalVariables|GetYearTemp) 1)))
  (bind _output_get (LocalVariables|SetDayOfTheWeek (+ (Math|Integer|%(Integer) (Math|Integer|Absolute(Integer) (+ (LocalVariables|GetDayTemp) (Math|Float|Truncate (* (LocalVariables|GetMonthTemp) 2.0)) (Math|Float|Truncate (/ (* (+ (LocalVariables|GetMonthTemp) 1) 3.0) 5.0)) (LocalVariables|GetYearTemp) (/ (LocalVariables|GetYearTemp) 4))) 7) 1)))
  (return _output_get))