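; Portal system actor that drives the view components of two linked portals so each follows the player camera as seen through the other.
; Every tick, Portal1Update and Portal2Update place the opposite portal's PortalView by mapping the player camera's transform from one portal's frame into the other's, flipped 180 degrees in yaw.
; Only Portal 2's view gets an extra fixed X offset; an AR pawn camera lookup is left unused.
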(event EventBeginPlay)

(event Collision|EventActorBeginOverlap
  (params (OtherActor :type Actor%20Object%20Reference)))

(event EventTick
  (params (DeltaSeconds :type Float%20%28single-precision%29))
  (CallFunction|Portal1Update)
  (CallFunction|Portal2Update))

(fn ConstructionScript)

(fn Portal1Update
  (bind _returnvalue (Game|GetPlayerCameraManager 0))
  (bind _portal1 (Variables|Default|GetPortal1))
  (bind _portal2 (Variables|Default|GetPortal2))
  (bind _defaultsceneroot (Variables|/Game/Blueprints/Portal/Portal2_BP.Portal2_BP_C|GetDefaultSceneRoot _portal2))
  (bind _defaultsceneroot_2 (Variables|/Game/Blueprints/Portal/Portal1_BP.Portal1_BP_C|GetDefaultSceneRoot _portal1))
  (bind _transformcomponent (Variables|/Script/Engine.PlayerCameraManager|GetTransformComponent _returnvalue))
  (bind _returnvalue_2 (Transformation|GetWorldRotation _defaultsceneroot))
  (bind _returnvalue_3 (Transformation|GetWorldLocation _transformcomponent))
  (bind _returnvalue_4 (Transformation|GetWorldLocation _defaultsceneroot))
  (bind _returnvalue_5 (Transformation|GetWorldRotation _defaultsceneroot_2))
  (bind _returnvalue_6 (Transformation|GetWorldLocation _defaultsceneroot_2))
  (bind _returnvalue_7 (- (.yaw _returnvalue_2) 1.8e+02))
  (bind _returnvalue_8 (Math|Rotator|MakeRotator (.roll _returnvalue_2) (.pitch _returnvalue_2) _returnvalue_7))
  (bind _returnvalue_9 (Math|Rotator|Delta(Rotator) _returnvalue_8 _returnvalue_5))
  (bind _returnvalue_10 (Math|Vector|RotateVector _returnvalue_6 _returnvalue_9))
  (bind _returnvalue_11 (Math|Vector|RotateVector _returnvalue_3 _returnvalue_9))
  (bind _returnvalue_12 (- _returnvalue_4 _returnvalue_10))
  (bind _returnvalue_13 (+ _returnvalue_12 _returnvalue_11))
  (Transformation|SetWorldLocationAndRotation (Variables|/Game/Blueprints/Portal/Portal2_BP.Portal2_BP_C|GetPortalView (Variables|Default|GetPortal2)) (Math|Vector|MakeVector (+ (.x _returnvalue_13) 2.5e+02) (.y _returnvalue_13) (.z _returnvalue_13)) (Math|Rotator|CombineRotators (Transformation|GetWorldRotation _transformcomponent) _returnvalue_9) false false))

(fn Portal2Update
  (bind _returnvalue (Game|GetPlayerCameraManager 0))
  (bind _portal1 (Variables|Default|GetPortal1))
  (bind _portal2 (Variables|Default|GetPortal2))
  (bind _defaultsceneroot (Variables|/Game/Blueprints/Portal/Portal2_BP.Portal2_BP_C|GetDefaultSceneRoot _portal2))
  (bind _defaultsceneroot_2 (Variables|/Game/Blueprints/Portal/Portal1_BP.Portal1_BP_C|GetDefaultSceneRoot _portal1))
  (bind _transformcomponent (Variables|/Script/Engine.PlayerCameraManager|GetTransformComponent _returnvalue))
  (bind _returnvalue_2 (Transformation|GetWorldRotation _defaultsceneroot_2))
  (bind _returnvalue_3 (Transformation|GetWorldRotation _defaultsceneroot))
  (bind _returnvalue_4 (- (.yaw _returnvalue_2) 1.8e+02))
  (bind _returnvalue_5 (Math|Rotator|MakeRotator (.roll _returnvalue_2) (.pitch _returnvalue_2) _returnvalue_4))
  (bind _returnvalue_6 (Math|Rotator|Delta(Rotator) _returnvalue_5 _returnvalue_3))
  (Transformation|SetWorldLocationAndRotation (Variables|/Game/Blueprints/Portal/Portal1_BP.Portal1_BP_C|GetPortalView (Variables|Default|GetPortal1)) (+ (- (Transformation|GetWorldLocation _defaultsceneroot_2) (Math|Vector|RotateVector (Transformation|GetWorldLocation _defaultsceneroot) _returnvalue_6)) (Math|Vector|RotateVector (Transformation|GetWorldLocation _transformcomponent) _returnvalue_6)) (Math|Rotator|CombineRotators (Transformation|GetWorldRotation _transformcomponent) _returnvalue_6) false false))